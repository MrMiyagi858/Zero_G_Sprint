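; Player character for an endless runner that auto-runs along its control yaw, strafes, and flips gravity on Jump.
; Jump, allowed only when a mesh-to-FloorCheck trace finds ground, rotates the actor, launches it and inverts GravityScale; the trace also switches Walking/Falling.
; When CanTurn is set, Left/Right change the target rotation by 90 degrees, which Tick interpolates toward.
; It also creates the HUD, accumulates distance on a timer, and shows GameOver after death.
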(event Custom|TurnCorner
  (bind _returnvalue (Pawn|GetControlRotation :!class /Script/Engine.Pawn))
  (bind _desiredrotation (Variables|Default|GetDesiredRotation))
  ;[1 1 1] Do corner turn
  (if (Utilities|Enum|NotEqual(Enum) _returnvalue _desiredrotation)
    (Pawn|SetControlRotation (Game|GetPlayerController 0) (Math|Interpolation|RInterpTo _returnvalue _desiredrotation (Utilities|Time|GetWorldDeltaSeconds) 1e+01))))

(event Custom|Add%20Distance
  ;[1 1 1] distants traveled
  (Variables|Default|SetTotal%20Distance%20Traveled (+ (Math|Vector|VectorLength (- (Variables|Default|GetLast%20Recorded%20Location) (Transformation|GetActorLocation))) (Variables|Default|GetTotal%20Distance%20Traveled)))
  (Variables|Default|SetLast%20Recorded%20Location (Transformation|GetActorLocation)))

(event Custom|Death
  ;[1 1 1] Death with restart
  (Variables|Default|SetIsDead? true)
  (Input|DisableInput 0)
  (Rendering|SetVisibility (Variables|Character|GetMesh) false false)
  (Utilities|FlowControl|Delay 3.0)
  (bind _returnvalue (UserInterface|CreateWidget "/Game/Joe/GameOver.GameOver_C"))
  (UserInterface|Viewport|AddtoViewport _returnvalue 0))

(event Custom|FollowCharacterRotation)

(event EventTick
  (params (DeltaSeconds :type Float%20%28single-precision%29))
  (bind _charactermovement (Variables|Character|GetCharacterMovement))
  ;[1 1 1] Endless Run
  (Utilities|FlowControl|Sequence
    (:then_0
      (if (not (Variables|Default|GetIsDead?))
        (CallFunction|TurnCorner)
        (Pawn|Input|AddMovementInput (Math|Vector|GetForwardVector (Math|Rotator|MakeRotator 0.0 0.0 (.Yaw (Math|Rotator|BreakRotator (Pawn|GetControlRotation :!class /Script/Engine.Pawn))))) 1.0 false)))
    (:then_1
      (bind (_outhit _returnvalue) (Collision|LineTraceByChannel (Transformation|GetWorldLocation (Variables|Character|GetMesh)) (Transformation|GetWorldLocation (Variables|Default|GetfloorCheck)) "TraceTypeQuery4" false 0 "None"))
      (if _returnvalue
        (Pawn|Components|CharacterMovement|SetMovementMode _charactermovement "MOVE_Walking" 0)
        (Variables|Default|Setisgrounded true)
        (else
          (Pawn|Components|CharacterMovement|SetMovementMode _charactermovement "MOVE_Falling" 0)
          (Variables|Default|Setisgrounded false))))))

(event EventBeginPlay
  ;[1 1 1] distants traveled
  (Utilities|FlowControl|Sequence
    (:then_0
      (Utilities|Time|SetTimerbyFunctionName 0 "Add Distance" 1.0 true)
      (Variables|Default|SetLast%20Recorded%20Location (Transformation|GetActorLocation)))
    (:then_1
      (bind _returnvalue (UserInterface|CreateWidget "/Game/Jared/UI/Run_HUD.Run_HUD_C"))
      (UserInterface|Viewport|AddtoViewport _returnvalue 0))))

(event Input|ActionEvents|InputActionJump
  (params (Key :type Key%20Structure))
  ;[1 1 1] camera switch
)

(event Input|ActionEvents|InputActionJump
  (params (Key :type Key%20Structure))
  (bind _returnvalue (Transformation|GetActorRotation))
  (bind _returnvalue_2 (Transformation|GetActorRotation))
  (bind (_roll _pitch _yaw) (Math|Rotator|BreakRotator _returnvalue))
  (bind (_roll_2 _pitch_2 _yaw_2) (Math|Rotator|BreakRotator _returnvalue_2))
  ;[1 1 1] Reverse Gravity
  (:Pressed
    (if (Variables|Default|Getisgrounded)
      (Development|PrintString "fliped")
      (if (Variables|Default|GetisgravityShifted?)
        (Transformation|SetActorRotation (Math|Rotator|MakeRotator _roll -1.8e+02 _yaw) true)
        (Character|LaunchCharacter "0, 0,-1000.000000" false false)
        (Variables|/Script/Engine.CharacterMovementComponent|SetGravityScale (Variables|Character|GetCharacterMovement) 1e+01)
        (Variables|Default|SetisgravityShifted? false)
        (else
          (Transformation|SetActorRotation (Math|Rotator|MakeRotator _roll_2 1.8e+02 _yaw_2) true)
          (Character|LaunchCharacter "0, 0,1000.000000" false false)
          (Variables|/Script/Engine.CharacterMovementComponent|SetGravityScale (Variables|Character|GetCharacterMovement) -1e+01)
          (Variables|Default|SetisgravityShifted? true))))))

(event Input|AxisEvents|InputAxisMoveRight
  (params (AxisValue :type Float%20%28single-precision%29))
  ;[1 1 1] Endless Run
  (Pawn|Input|AddMovementInput (Math|Vector|GetRightVector (Math|Rotator|MakeRotator 0.0 0.0 (.Yaw (Math|Rotator|BreakRotator (Pawn|GetControlRotation :!class /Script/Engine.Pawn))))) AxisValue false))

(event Input|KeyboardEvents|Left
  (params (Key :type Key%20Structure))
  ;[1 0.9042 0.2499] A & D input for corners
  (:Pressed
    (if (Variables|Default|GetCanTurn)
      (Variables|Default|SetDesiredRotation (Math|Rotator|CombineRotators (Variables|Default|GetDesiredRotation) "0,-90.000000, 0"))
      (Variables|Default|SetCanTurn false))))

(event Input|KeyboardEvents|Right
  (params (Key :type Key%20Structure))
  ;[1 0.9042 0.2499] A & D input for corners
  (:Pressed
    (if (Variables|Default|GetCanTurn)
      (Variables|Default|SetDesiredRotation (Math|Rotator|CombineRotators (Variables|Default|GetDesiredRotation) "0,90.000000, 0"))
      (Variables|Default|SetCanTurn false))))

(fn ConstructionScript)