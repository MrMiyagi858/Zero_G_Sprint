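; Floor tile for an endless runner that keeps the track going as the RunCharacter advances.
; Overlapping EndTrigger calls AddFloorTile on Run_GameMode, then destroys this tile after a short delay.
; GetAttachTransform exposes the AttachArrow's world transform as the location for the next piece.
; Wall-impact death checks and random coin and blocker spawning are present only as disconnected logic, so none of them run.
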(event OnComponentBeginOverlap(EndTrigger)
  (params (OverlappedComponent :type Primitive%20Component%20Object%20Reference) (OtherActor :type Actor%20Object%20Reference) (OtherComp :type Primitive%20Component%20Object%20Reference) (OtherBodyIndex :type Integer) (bFromSweep :type Boolean) (SweepResult :type Hit%20Result%20Structure%20%28by%20ref%29))
  ;[1 1 1] Adding/Deleting Map Tiles
  (Utilities|Casting|CastToRunCharacter OtherActor)
  (bind _asrun_game_mode (Utilities|Casting|CastToRun_GameMode (Game|GetGameMode)))
  (Default|AddFloorTile _asrun_game_mode)
  (Utilities|FlowControl|Delay 2.0)
  (Actor|DestroyActor))

(event OnComponentHit(Right_Wall)
  (params (HitComponent :type Primitive%20Component%20Object%20Reference) (OtherActor :type Actor%20Object%20Reference) (OtherComp :type Primitive%20Component%20Object%20Reference) (NormalImpulse :type Vector :default "0, 0, 0") (Hit :type Hit%20Result%20Structure%20%28by%20ref%29)))

(event OnComponentHit(Left_Wall)
  (params (HitComponent :type Primitive%20Component%20Object%20Reference) (OtherActor :type Actor%20Object%20Reference) (OtherComp :type Primitive%20Component%20Object%20Reference) (NormalImpulse :type Vector :default "0, 0, 0") (Hit :type Hit%20Result%20Structure%20%28by%20ref%29)))

(event EventBeginPlay)

(event Collision|EventActorBeginOverlap
  (params (OtherActor :type Actor%20Object%20Reference)))

(event EventTick
  (params (DeltaSeconds :type Float%20%28single-precision%29)))

(fn ConstructionScript
  ;[1 1 1] Random generator
)

(fn GetAttachTransform
  ;[1 1 1] Getting location of next tile piece
  (return (Transformation|GetWorldTransform (Variables|Default|GetAttach%20Arrow))))

(fn SetSpawnPoints
  ;[1 1 1] Setting spawn points
)

(fn SpawnBlocker
  ;[1 1 1] Obstacle generator for spawn points
)

(fn SpawnCoins)