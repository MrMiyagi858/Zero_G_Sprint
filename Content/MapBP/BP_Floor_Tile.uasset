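; BP_Floor_Tile is an endless-runner floor segment that carries a randomly placed obstacle.
; The construction script gathers left, middle and right spawn point transforms and adds a child-actor blocker at one chosen at random.
; When the RunCharacter overlaps EndTrigger, the tile calls AddFloorTile on Run_GameMode, then destroys itself after a short delay.
; GetAttachTransform exposes the AttachArrow world transform as the location of the next tile.
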(event OnComponentBeginOverlap(EndTrigger)
  (params (OverlappedComponent :type Primitive%20Component%20Object%20Reference) (OtherActor :type Actor%20Object%20Reference) (OtherComp :type Primitive%20Component%20Object%20Reference) (OtherBodyIndex :type Integer) (bFromSweep :type Boolean) (SweepResult :type Hit%20Result%20Structure%20%28by%20ref%29))
  ;[1 1 1] Adding/Deleting Map Tiles
  (Utilities|Casting|CastToRunCharacter OtherActor)
  (bind _asrun_game_mode (Utilities|Casting|CastToRun_GameMode (Game|GetGameMode)))
  (Default|AddFloorTile _asrun_game_mode)
  (Utilities|FlowControl|Delay 2.0)
  (Actor|DestroyActor))

(event EventBeginPlay)

(event Collision|EventActorBeginOverlap
  (params (OtherActor :type Actor%20Object%20Reference)))

(event EventTick
  (params (DeltaSeconds :type Float%20%28single-precision%29)))

(fn ConstructionScript
  ;[1 1 1] Tile pieces that spawn with obstacles
  (CallFunction|SetSpawnPoints)
  (CallFunction|SpawnBlocker))

(fn GetAttachTransform
  ;[1 1 1] Getting location of next tile piece
  (return (Transformation|GetWorldTransform (Variables|Default|GetAttach_Arrow))))

(fn SetSpawnPoints
  ;[1 1 1] Setting for random three spawn points
  (Variables|Default|SetSpawnPoints (Utilities|Array|MakeArray (Transformation|GetRelativeTransform (Variables|Default|GetSpawn_Point_Left)) (Transformation|GetRelativeTransform (Variables|Default|GetSpawn_Point_Middle)) (Transformation|GetRelativeTransform (Variables|Default|GetSpawn_Point_Right)))))

(fn SpawnBlocker
  (bind _spawnpoints (Variables|Default|GetSpawnPoints))
  ;[1 1 1] Obstacle generator for spawn points
  (AddComponent|AddChildActorComponent false (Utilities|Array|Get(acopy) _spawnpoints (Math|Random|RandomIntegerinRange 0 (Utilities|Array|LastIndex _spawnpoints)))))