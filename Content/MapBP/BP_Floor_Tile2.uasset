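; Floor tile for an endless runner that asks Run_GameMode to add a tile when RunCharacter reaches EndTrigger, then destroys itself after a short delay.
; AttachArrow supplies the next tile's transform, and construction randomly decides whether to scatter coin child actors in floor and ceiling boxes.
; Side walls kill the runner when the hit normal matches its forward vector.
; Obstacle spawning is disconnected, though spawn points are still recorded.
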(event OnComponentBeginOverlap(EndTrigger)
  (params (OverlappedComponent :type Primitive%20Component%20Object%20Reference) (OtherActor :type Actor%20Object%20Reference) (OtherComp :type Primitive%20Component%20Object%20Reference) (OtherBodyIndex :type Integer) (bFromSweep :type Boolean) (SweepResult :type Hit%20Result%20Structure%20%28by%20ref%29))
  ;[1 1 1] Adding/Deleting Map Tiles
  (Utilities|Casting|CastToRunCharacter OtherActor)
  (bind _asrun_game_mode (Utilities|Casting|CastToRun_GameMode (Game|GetGameMode)))
  (Default|AddFloorTile _asrun_game_mode)
  (Utilities|FlowControl|Delay 2.0)
  (Actor|DestroyActor))

(event OnComponentHit(Right_Wall)
  (params (HitComponent :type Primitive%20Component%20Object%20Reference) (OtherActor :type Actor%20Object%20Reference) (OtherComp :type Primitive%20Component%20Object%20Reference) (NormalImpulse :type Vector :default "0, 0, 0") (Hit :type Hit%20Result%20Structure%20%28by%20ref%29))
  (bind _asrun_character (Utilities|Casting|CastToRunCharacter OtherActor))
  (if (Math|Float|NearlyEqual(Float) (Math|Vector|DotProduct (.normal Hit) (Transformation|GetActorForwardVector _asrun_character)) 1.0 1e-06)
    (Default|Death _asrun_character)))

(event OnComponentHit(Left_Wall)
  (params (HitComponent :type Primitive%20Component%20Object%20Reference) (OtherActor :type Actor%20Object%20Reference) (OtherComp :type Primitive%20Component%20Object%20Reference) (NormalImpulse :type Vector :default "0, 0, 0") (Hit :type Hit%20Result%20Structure%20%28by%20ref%29))
  (bind _asrun_character (Utilities|Casting|CastToRunCharacter OtherActor))
  (if (Math|Float|NearlyEqual(Float) (Math|Vector|DotProduct (.normal Hit) (Transformation|GetActorForwardVector _asrun_character)) 1.0 1e-06)
    (Default|Death _asrun_character)))

(event EventBeginPlay)

(event Collision|EventActorBeginOverlap
  (params (OtherActor :type Actor%20Object%20Reference)))

(event EventTick
  (params (DeltaSeconds :type Float%20%28single-precision%29)))

(fn ConstructionScript
  ;[1 1 1] Random generator
  (CallFunction|SetSpawnPoints)
  (switch int (Math|Random|RandomIntegerinRange 0 1)
    (:1
      (CallFunction|SpawnCoins))))

(fn GetAttachTransform
  ;[1 1 1] Getting location of next tile piece
  (return (Transformation|GetWorldTransform (Variables|Default|GetAttach_Arrow))))

(fn SetSpawnPoints
  ;[1 1 1] Setting spawn points
  (Utilities|FlowControl|Sequence
    (:then_0
      (Variables|Default|SetSpawnPoints (Utilities|Array|MakeArray (Transformation|GetRelativeTransform (Variables|Default|GetSpawn_Point_Middle2)))))
    (:then_1
      (Variables|Default|SetSpawnPoints2 (Utilities|Array|MakeArray (Transformation|GetRelativeTransform (Variables|Default|GetCeiling_Spawn_Point_Middle2)))))))

(fn SpawnBlocker
  ;[1 1 1] Obstacle generator for spawn points
)

(fn SpawnCoins
  (bind _coinarea (Variables|Default|GetCoinArea))
  (bind _coinareaceiling (Variables|Default|GetCoinAreaCeiling))
  (Utilities|FlowControl|Sequence
    (:then_0
      (for _index (range 0 3)
        (AddComponent|AddChildActorComponent false (Math|Conversions|ToTransform(Vector) (Math|Random|RandomPointinBoundingBox (Variables|/Script/Engine.SceneComponent|GetRelativeLocation _coinarea) (Variables|/Script/Engine.BoxComponent|GetBoxExtent _coinarea))))))
    (:then_1
      (for _index_2 (range 0 3)
        (AddComponent|AddChildActorComponent false (Math|Conversions|ToTransform(Vector) (Math|Random|RandomPointinBoundingBox (Variables|/Script/Engine.SceneComponent|GetRelativeLocation _coinareaceiling) (Variables|/Script/Engine.BoxComponent|GetBoxExtent _coinareaceiling))))))))